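; BP_info_4 is a VR-style grabbable info actor that reacts to the left and right grab input actions.
; Either grab press adds a GrabComponent to the Plane's owner and, if Plane is tagged "info", advances the "info" achievement.
; The actor is destroyed when left grab completes or right grab is canceled.
; The input handlers run without any overlap or held-object check.
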(event `EnhancedInput|/Game/VRTemplate/Input/Actions/IA_Grab_Left`
  (params (ActionValue :type "Float (double-precision)") (ElapsedSeconds :type "Float (double-precision)") (TriggeredSeconds :type "Float (double-precision)") (InputAction :type "InputAction Object Reference" :default "/Game/VRTemplate/Input/Actions/IA_Grab_Left.IA_Grab_Left"))
  (:`Started`
    (`AddComponent|NODE_AddGrabComponent-0` :`self` (`ActorComponent.GetOwner` (`self.Plane`)) :!label _label)
    (if (`ActorComponent.ComponentHasTag` (`self.Plane`) "info")
      (`AchievementSubSystem.AddAchievementProgress` (subsystem `AchievementSubSystem`) "info" 1.0)))
  (:`Completed`
    (`self.K2_DestroyActor` (`ActorComponent.GetOwner` (`self.Plane`)) :!label _label_2)))

(event `EnhancedInput|/Game/VRTemplate/Input/Actions/IA_Grab_Right`
  (params (ActionValue :type "Float (double-precision)") (ElapsedSeconds :type "Float (double-precision)") (TriggeredSeconds :type "Float (double-precision)") (InputAction :type "InputAction Object Reference" :default "/Game/VRTemplate/Input/Actions/IA_Grab_Right.IA_Grab_Right"))
  (:`Started`
    (goto _label))
  (:`Canceled`
    (goto _label_2)))

(fn `UserConstructionScript`)